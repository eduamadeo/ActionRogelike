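; Explosive barrel actor that blows up automatically a few seconds after play begins.
; The authority starts a one-shot timer on BeginPlay, which calls a multicast explode event and then sets a short lifespan for delayed destruction.
; The multicast event fires the radial force impulse, hides the actor and disables its collision.
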(event `self.ReceiveBeginPlay`
  (if (`self.HasAuthority`)
    (`KismetSystemLibrary.K2_SetTimerDelegate` (delegate `Explode`) 4.0)))

(event `Explode`
  (`self.MulticastExplode`)
  (`self.SetLifeSpan` 2.0))

(event `MulticastExplode`
  (`RadialForceComponent.FireImpulse` (`self.RadialForceComp`))
  (`self.SetActorHiddenInGame` true)
  (`self.SetActorEnableCollision` false))

(fn `UserConstructionScript`)