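; BlackholeProjectileBP is a black hole projectile that destroys actors it hits.
; On BeginPlay, its SphereComp ignores the instigator while moving.
; A separate component named Destroy handles hit events and destroys the other actor unless it is the instigator.
; The projectile's lifetime follows EffectComp, as it destroys itself when that particle system finishes.
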(event `self.ReceiveBeginPlay`
  (`PrimitiveComponent.IgnoreActorWhenMoving` (`self.SphereComp`) (`self.GetInstigator`) true)
  (add `ParticleSystemComponent.OnSystemFinished` (`self.EffectComp`) (delegate `OnSystemFinished_Particle`)))

(event `OnSystemFinished_Particle`
  (params (PSystem :type "ParticleSystemComponent Object Reference"))
  (`self.K2_DestroyActor`))

(event `self.Destroy.OnComponentHit`
  (params (HitComponent :type "PrimitiveComponent Object Reference") (OtherActor :type "Actor Object Reference") (OtherComp :type "PrimitiveComponent Object Reference") (NormalImpulse :type "Vector Structure") (Hit :type "HitResult Structure (by ref)"))
  (if (!= OtherActor (`self.GetInstigator`))
    (`self.K2_DestroyActor` OtherActor)))

(fn `UserConstructionScript`)